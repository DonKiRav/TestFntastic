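; BP_MainNest is a nest actor that spawns minions, which the author's comment calls "turtles".
; FunctionSpawnMinion spawns MinionClass slightly above SpawnPoint, passing EndPoint as the target, itself as the start point and MinionTipe as the BT parameter.
; It also plays a 2D spawn sound and spawns a BP_ky_fireStorm effect at SpawnPoint.
; The event graph and construction script are empty, so nothing in this Blueprint calls the function.
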(fn `Function_SpawnMinion`
  ;[1 1 1] Спавним "черепашку", звук и визуальный эффект
  (`|SpawnActorFromClass` (`self.MinionClass`) (`KismetMathLibrary.MakeTransform` (+ (`SceneComponent.K2_GetComponentLocation` (`self.SpawnPoint`)) (0.0 0.0 10.0))) "Undefined" "OverrideRootScale" null (`self.EndPoint`) (`self.MinionTipe`) self null)
  (`GameplayStatics.PlaySound2D` "/Game/MainFolder/Sound/Cue_Spawn.Cue_Spawn" 1.0 1.0 0.0 null null)
  (`|SpawnActorFromClass` "/Game/FXVarietyPack/Blueprints/BP_ky_fireStorm.BP_ky_fireStorm_C" (`KismetMathLibrary.MakeTransform` (`SceneComponent.K2_GetComponentLocation` (`self.SpawnPoint`))) "Undefined" "OverrideRootScale" null null))

(fn `UserConstructionScript`)