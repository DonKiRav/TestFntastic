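; BP_MainButton is a numbered button that makes its Nest spawn a minion ("turtle") when the player touches it.
; On BeginPlay it passes its Index to the WD_ShowNumber widget on its Widget component for display.
; Box overlaps from actors tagged Player call FunctionSpawnMinion on Nest, gated by a DoOnce that resets after a one-second delay as a cooldown.
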(event `self.ReceiveBeginPlay`
  ;[1 1 1] Передаем в виджет число
  (bind _aswd_show_number (cast `/Game/MainFolder/UI/WD_ShowNumber` (`WidgetComponent.GetWidget` (`self.Widget`))))
  (`/Game/MainFolder/UI/WD_ShowNumber.Function_SetNumber` _aswd_show_number (`self.Index`)))

(event `self.Box.OnComponentBeginOverlap`
  (params (OverlappedComponent :type "PrimitiveComponent Object Reference") (OtherActor :type "Actor Object Reference") (OtherComp :type "PrimitiveComponent Object Reference") (OtherBodyIndex :type Integer) (bFromSweep :type Boolean) (SweepResult :type "HitResult Structure (by ref)"))
  ;[1 1 1] Если игрок соприкасается с кнопкой - спавним "черепашку"
  (if (`self.ActorHasTag` OtherActor "Player")
    (`/Engine/EditorBlueprintResources/StandardMacros.DoOnce` false :!label _label
      (:`Completed`
        (`/Game/MainFolder/Nests/BP_MainNest.Function_SpawnMinion` (`self.Nest`))
        (`KismetSystemLibrary.Delay` 1.0)
        (goto _label :!via `Reset`)))))

(fn `UserConstructionScript`)